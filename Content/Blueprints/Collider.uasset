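; Collider is a debug test Blueprint for inspecting collision channels and overlap events on a Box component.
; At BeginPlay it sets the box to ignore the Pawn channel, then prints the box's collision object type, naming only World Static, World Dynamic or Pawn.
; The box's begin-overlap event prints a "COLLIDED" message to show when an overlap still fires.
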(event `self.ReceiveBeginPlay`
  (bind _box (`self.Box`))
  (`PrimitiveComponent.SetCollisionResponseToChannel` _box "ECC_Pawn" "ECR_Ignore")
  (switch `ECollisionChannel` (`PrimitiveComponent.GetCollisionObjectType` _box)
    (:`ECC_WorldStatic`
      (set `self.Coll` "WorldStatic"))
    (:`ECC_WorldDynamic`
      (set `self.Coll` "WorldDynamic"))
    (:`ECC_Pawn`
      (set `self.Coll` "Pawn")))
  (`KismetSystemLibrary.PrintString` (`KismetStringLibrary.Concat_StrStr` "Collision Object Typeby default is :::" (`self.Coll`)) true true (struct :`R` 1.0 :`B` 0.838456 :`A` 1.0) 20.0))

(event `self.Box.OnComponentBeginOverlap`
  (params (OverlappedComponent :type "PrimitiveComponent Object Reference") (OtherActor :type "Actor Object Reference") (OtherComp :type "PrimitiveComponent Object Reference") (OtherBodyIndex :type Integer) (bFromSweep :type Boolean) (SweepResult :type "HitResult Structure (by ref)"))
  (`KismetSystemLibrary.PrintString` "COLLIDED!!!!!!!!!!!!!!!!!!!!!!!!!!!!!!!!!!!!!"))

(fn `UserConstructionScript`)