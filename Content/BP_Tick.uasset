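; BP_Tick is a character Blueprint that nudges itself back and forth through its movement component every frame.
; Tick makes two opposite, swept diagonal moves at the current rotation, so net displacement is zero unless a sweep is blocked.
; An unconnected boolean check compares camera boom yaw and pitch with mesh rotation ranges, and the construction script is empty.
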(event `self.ReceiveTick`
  (params (DeltaSeconds :type "Float (single-precision)"))
  (bind _returnvalue (`self.K2_GetActorRotation`))
  (bind _charactermovement (`self.CharacterMovement`))
  (`MovementComponent.K2_MoveUpdatedComponent` _charactermovement (1.0 1.0 0.0) _returnvalue true false)
  (`MovementComponent.K2_MoveUpdatedComponent` _charactermovement (-1.0 -1.0 0.0) _returnvalue true false))

(fn `UserConstructionScript`)