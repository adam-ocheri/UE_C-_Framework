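; HUD Blueprint that draws a single test-like rectangle over the lower-right quarter of the screen.
; BeginPlay turns on ShowHUD, and DrawHUD redraws the rectangle from a small offset past screen center to the right and bottom edges.
; Unconnected DrawLine and selection-rectangle nodes remain in the graph but never run.
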(event `self.ReceiveBeginPlay`
  (set `self.bShowHUD` true))

(event `self.ReceiveDrawHUD`
  (params (SizeX :type Integer) (SizeY :type Integer))
  (bind _returnvalue (`KismetMathLibrary.Conv_IntToDouble` (/ SizeX 2)))
  (bind _returnvalue_2 (`KismetMathLibrary.Conv_IntToDouble` (/ SizeY 2)))
  (`self.DrawRect` (struct :`A` 1) (+ _returnvalue 10.0) (+ _returnvalue_2 10.0) (+ _returnvalue -10.0) (+ _returnvalue_2 -10.0)))

(fn `UserConstructionScript`)