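; BP_MyHUD is a HUD Blueprint that attempts to draw a brush-filled box on DrawHUD.
; The box starts at screen center and is sized to the full screen, so it would extend past the bottom-right edges.
; It calls the UMG paint DrawBox with a freshly made, empty PaintContext instead of drawing on the HUD canvas.
; All other events and the construction script are empty.
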(event `self.ReceiveDrawHUD`
  (params (SizeX :type Integer) (SizeY :type Integer))
  (`WidgetBlueprintLibrary.DrawBox` (make `PaintContext`) (`KismetMathLibrary.MakeVector2D` (`KismetMathLibrary.Conv_IntToDouble` (/ SizeX 2)) (`KismetMathLibrary.Conv_IntToDouble` (/ SizeY 2))) (`KismetMathLibrary.MakeVector2D` (`KismetMathLibrary.Conv_IntToDouble` SizeX) (`KismetMathLibrary.Conv_IntToDouble` SizeY)) (`self.Brush`)))

(fn `UserConstructionScript`)